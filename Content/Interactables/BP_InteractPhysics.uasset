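; BP_InteractPhysics is a colored physics cube the player picks up and drops through interact events.
; INTInteract, only if the player is not already holding, sets IsHolding, disables the cube's physics and collision, and snaps it to ArrowAttach.
; INTDrop detaches it in world space and restores collision and physics, without clearing IsHolding itself.
; The construction script tints the cube with PickupColor through a dynamic material instance.
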(event EventINTInteract
  (params (PlayerRef :type BP%20Player%20Char%20Object%20Reference))
  (bind _cube (Variables|Default|GetCube))
  ;[1 1 1] Attach
  (if (not (Variables|/Game/Player/BP_PlayerChar.BP_PlayerChar_C|GetisHolding PlayerRef))
    (Variables|/Game/Player/BP_PlayerChar.BP_PlayerChar_C|SetisHolding PlayerRef true)
    (Physics|SetSimulatePhysics _cube false)
    (Collision|SetCollisionEnabled _cube "NoCollision")
    (Transformation|AttachComponentToComponent (Variables|Default|GetCube) (Variables|/Game/Player/BP_PlayerChar.BP_PlayerChar_C|GetArrowAttach PlayerRef) "None" "SnapToTarget" "KeepRelative" "KeepRelative" false)))

(event EventINTDrop
  (bind _cube (Variables|Default|GetCube))
  ;[1 1 1] Detach
  (Transformation|DetachFromActor "KeepWorld" "KeepWorld" "KeepWorld")
  (Collision|SetCollisionEnabled _cube "QueryAndPhysics")
  (Physics|SetSimulatePhysics _cube true))

(fn ConstructionScript
  (bind _returnvalue (Rendering|Material|CreateDynamicMaterialInstance (Variables|Default|GetCube) 0 "/Game/Interactables/InteractableMaterials/MAT_BaseColor.MAT_BaseColor" "None" :!class /Script/Engine.PrimitiveComponent))
  (bind _output_get (Variables|Default|SetColorDMI _returnvalue))
  (Rendering|Material|SetVectorParameterValue _output_get "BaseColor" (Variables|Default|GetPickupColor) :!class /Script/Engine.MaterialInstanceDynamic))