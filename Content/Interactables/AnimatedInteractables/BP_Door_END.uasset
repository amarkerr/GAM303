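; BP_Door_END is an interactable end-of-game door that, when unlocked, congratulates the player and quits the game.
; Interacting while locked deals damage to the player character.
; When unlocked, it plays a timeline whose update prints the message, zeroes the Arrow's rotation and quits after a delay; the player-side swing angle it computes is unused.
; The construction script tints the Cube through a dynamic material instance using PickupColor.
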(event EventINTInteract
  (params (PlayerRef :type BP%20Player%20Char%20Object%20Reference))
  ;[1 1 1] Open
  (if (Variables|Default|GetisUnlocked)
    (CallFunction|UpdateDoorAngle2 PlayerRef)
    (Timeline|Timeline Play
      (:Update
        (Transformation|SetRelativeRotation (Variables|Default|GetArrow) (Math|Rotator|MakeRotator 0.0 0.0 0.0) false false)
        (Development|PrintString "CONGRATULATIONS")
        (Utilities|FlowControl|Delay 3.0)
        (Game|QuitGame 0 "Quit" false)))
    (else
      (Game|Damage|ApplyDamage (Game|GetPlayerCharacter 0) 1e+01 0 0))))

(fn ConstructionScript
  (bind _returnvalue (Rendering|Material|CreateDynamicMaterialInstance (Variables|Default|GetCube) 0 "/Game/Interactables/InteractableMaterials/MAT_BaseColor.MAT_BaseColor" "None" :!class /Script/Engine.PrimitiveComponent))
  (bind _output_get (Variables|Default|SetColorDMI _returnvalue))
  (Rendering|Material|SetVectorParameterValue _output_get "BaseColor" (Variables|Default|GetPickupColor) :!class /Script/Engine.MaterialInstanceDynamic))

(fn UpdateDoorAngle2
  (params (self2 :type Actor%20Object%20Reference))
  (return (select (> (Math|Vector|DotProduct (Math|Vector|GetUnitDirection(Vector) (Transformation|GetActorLocation) (Transformation|GetActorLocation self2)) (Transformation|GetActorForwardVector)) 0.0) 9e+01 -9e+01)))