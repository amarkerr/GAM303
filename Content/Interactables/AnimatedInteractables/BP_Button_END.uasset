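; BP_Button_END is a colored pressure button that unlocks a linked TargetDoor while a matching BP_InteractPhysics object rests on it.
; With DoesUnlock set, a PickupColor match unlocks the door, plays a sound and lowers the button by timeline.
; Any BP_InteractPhysics leaving relocks the door and reverses that timeline; without DoesUnlock, any overlap just plays a separate press animation.
; The construction script tints the button with PickupColor through a dynamic material.
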(event OnComponentBeginOverlap(Overlap)
  (params (OverlappedComponent :type Primitive%20Component%20Object%20Reference) (OtherActor :type Actor%20Object%20Reference) (OtherComp :type Primitive%20Component%20Object%20Reference) (OtherBodyIndex :type Integer) (bFromSweep :type Boolean) (SweepResult :type Hit%20Result%20Structure%20%28by%20ref%29))
  (bind _targetdoor (Variables|Default|GetTargetDoor))
  ;[1 1 1] Button Press/Door Open
  (if (Variables|Default|GetdoesUnlock)
    (bind _asbp_interact_physics (Utilities|Casting|CastToBP_InteractPhysics OtherActor))
    (if (== (Variables|/Game/Interactables/BP_InteractPhysics.BP_InteractPhysics_C|GetPickupColor _asbp_interact_physics) (Variables|Default|GetPickupColor))
      (Utilities|IsValid _targetdoor
        (:Is%20Valid
          (Variables|/Game/Interactables/AnimatedInteractables/BP_Door_END.BP_Door_END_C|SetisUnlocked _targetdoor true)
          (Audio|PlaySoundatLocation 0 (Transformation|GetActorLocation (Variables|Default|GetTargetDoor)) "0, 0, 0" 1.0 1.0 0.0 0 0 0 0)
          (Development|PrintString "Door is unlocked")
          (bind _alphatrack (Timeline|Alpha Play)
            (:Update
              (Transformation|SetRelativeLocation (Variables|Default|GetButton) (Math|Vector|MakeVector 0.0 0.0 (Math|Float|Lerp 5.0 1.0 _alphatrack)) false false))))
        (:Is%20Not%20Valid
          (Development|PrintString "Door not linked"))))
    (else
      (bind _alphatrack_2 (Timeline|Timeline Play)
        (:Update
          (Transformation|SetRelativeLocation (Variables|Default|GetButton) (Math|Vector|MakeVector 0.0 0.0 (Math|Float|Lerp 5.0 1.0 _alphatrack_2)) false false))))))

(event OnComponentEndOverlap(Overlap)
  (params (OverlappedComponent :type Primitive%20Component%20Object%20Reference) (OtherActor :type Actor%20Object%20Reference) (OtherComp :type Primitive%20Component%20Object%20Reference) (OtherBodyIndex :type Integer))
  ;[1 1 1] Button Press/Door Open
  (Utilities|Casting|CastToBP_InteractPhysics OtherActor)
  (Variables|/Game/Interactables/AnimatedInteractables/BP_Door_END.BP_Door_END_C|SetisUnlocked (Variables|Default|GetTargetDoor) false)
  (bind _alphatrack (Timeline|Alpha Reverse)
    (:Update
      (Transformation|SetRelativeLocation (Variables|Default|GetButton) (Math|Vector|MakeVector 0.0 0.0 (Math|Float|Lerp 5.0 1.0 _alphatrack)) false false))))

(fn ConstructionScript
  (bind _returnvalue (Rendering|Material|CreateDynamicMaterialInstance (Variables|Default|GetButton) 0 "/Game/Interactables/InteractableMaterials/MAT_BaseColor.MAT_BaseColor" "None" :!class /Script/Engine.PrimitiveComponent))
  (bind _output_get (Variables|Default|SetColorDMI _returnvalue))
  (Rendering|Material|SetVectorParameterValue _output_get "BaseColor" (Variables|Default|GetPickupColor) :!class /Script/Engine.MaterialInstanceDynamic))