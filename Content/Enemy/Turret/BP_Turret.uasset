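; BP_Turret is an enemy turret that aims and fires at the player while they are inside its detection box.
; Box overlap with BP_PlayerChar starts two looping timers, one for aiming and a faster one for firing, and leaving the box clears both.
; Aiming snaps PivotArrow toward player character 0 at each tick of its timer rather than every frame.
; Firing spawns BP_TurProj at ProjectileArrow's world transform.
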(event OnComponentBeginOverlap(Box)
  (params (OverlappedComponent :type Primitive%20Component%20Object%20Reference) (OtherActor :type Actor%20Object%20Reference) (OtherComp :type Primitive%20Component%20Object%20Reference) (OtherBodyIndex :type Integer) (bFromSweep :type Boolean) (SweepResult :type Hit%20Result%20Structure%20%28by%20ref%29))
  ;[1 1 1] Overlap Events
  (Utilities|Casting|CastToBP_PlayerChar OtherActor)
  (Utilities|Time|SetTimerbyFunctionName 0 "FollowPlayer" 0.5 true)
  (Utilities|Time|SetTimerbyFunctionName 0 "FireAtPlayer" 0.2 true))

(event OnComponentEndOverlap(Box)
  (params (OverlappedComponent :type Primitive%20Component%20Object%20Reference) (OtherActor :type Actor%20Object%20Reference) (OtherComp :type Primitive%20Component%20Object%20Reference) (OtherBodyIndex :type Integer))
  ;[1 1 1] Overlap Events
  (Utilities|Casting|CastToBP_PlayerChar OtherActor)
  (Utilities|Time|ClearTimerbyFunctionName 0 "FollowPlayer")
  (Utilities|Time|ClearTimerbyFunctionName 0 "FireAtPlayer"))

(event Custom|FollowPlayer
  ;[1 1 1] Turrent Follow Player
  (Transformation|SetWorldRotation (Variables|Default|GetPivotArrow) (Math|Rotator|FindLookatRotation (Transformation|GetActorLocation) (Transformation|GetActorLocation (Game|GetPlayerCharacter 0))) false false))

(event Custom|FireAtPlayer
  ;[1 1 1] Turret Fire
  (Game|SpawnActorfromClass "/Game/Enemy/Turret/BP_TurProj.BP_TurProj_C" (Transformation|GetWorldTransform (Variables|Default|GetProjectileArrow)) "Undefined" "MultiplyWithRoot" 0 0))

(fn ConstructionScript)